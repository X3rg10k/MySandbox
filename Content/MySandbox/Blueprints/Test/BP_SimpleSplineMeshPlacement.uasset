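; Spline-based placement Blueprint that fills an Instanced Static Mesh with evenly spaced copies of a chosen mesh along its spline.
; The construction script derives spacing from a placement offset, optionally plus the mesh's X bounds, and fits the instance count to the spline length.
; Each instance is unrotated, aimed at the next position, or aligned to the spline's rotation, with NoRotation overriding FindRotationFromNextMeshPos.
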(fn `GetLocationAtIndex`
  (params (AtIndex :type Integer))
  (returns (ReturnValue :type "Vector Structure"))
  (return (`SplineComponent.GetLocationAtDistanceAlongSpline` (`self.Spline`) (* AtIndex (`self.Spacing`)) "Local")))

(fn `UserConstructionScript`
  (locals (NumOfInstances :type Integer :default 0))
  (bind (_min _max) (break `Box` (`StaticMesh.GetBoundingBox` (`self.PlacedInstancedStaticMesh`))))
  (`|ExecutionSequence`
    (:`then_0`
      (bind _placedinstancedstaticmesh (`self.PlacedInstancedStaticMesh`)
        (:`then`
          (`StaticMeshComponent.SetStaticMesh` (`self.InstancedStaticMesh`) _placedinstancedstaticmesh))
        (:`else`)))
    (:`then_1`
      (`|ExecutionSequence`
        (:`then_0`
          (set `self.Spacing` (+ (`KismetMathLibrary.SelectFloat` (.x (- _max _min)) 0.0 (`self.bOffsetIncludingMeshBounds`)) (`self.PlacementOffset`)))
          (if (`self.bNoRotation`)
            (set `self.bFindRotationFromNextMeshPos` false)
            (elif (`self.bFindRotationFromNextMeshPos`)
              (set `self.bNoRotation` false))))
        (:`then_1`
          (bind _output_get (set `local.NumOfInstances` (`KismetMathLibrary.FFloor` (/ (`SplineComponent.GetSplineLength` (`self.Spline`)) (`self.Spacing`)))))
          (for _index (range (+ _output_get 1))
            (bind _returnvalue (`self.GetLocationAtIndex` _index))
            (`InstancedStaticMeshComponent.AddInstance` (`self.InstancedStaticMesh`) (`KismetMathLibrary.MakeTransform` _returnvalue (`KismetMathLibrary.SelectRotator` (struct) (`KismetMathLibrary.SelectRotator` (`KismetMathLibrary.MakeRotFromX` (- (`self.GetLocationAtIndex` (+ _index 1)) _returnvalue)) (`SplineComponent.GetRotationAtDistanceAlongSpline` (`self.Spline`) (* _index (`self.Spacing`)) "Local") (`self.bFindRotationFromNextMeshPos`)) (`self.bNoRotation`))) false)))))))