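; BP_CircleSpline is a test Blueprint that procedurally builds a closed circular spline from Segments and Radius.
; Its construction script clears the spline, then places local-space points on the XY plane using sine and cosine of each index's mapped angle.
; The angle range stops one segment short of 360 degrees, so the closed loop supplies the final segment.
; The spline updates once, after all points are added.
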(fn ConstructionScript
  (Spline|SetClosedLoop (Variables|Default|GetCircleSpline) true false)
  (Spline|ClearSplinePoints (Variables|Default|GetCircleSpline) false)
  (if (> (Variables|Settings|GetSegments) 0)
    (LocalVariables|SetActiveSegments (- (Variables|Settings|GetSegments) 1)) ; last segment in closed loop\nnot counted
    (for _index (range 0 (LocalVariables|GetActiveSegments))
      (LocalVariables|SetSegmentOfCircumference (Math|Float|MapRangeClamped (Math|Conversions|ToFloat(Integer) _index) 0.0 (Math|Conversions|ToFloat(Integer) (LocalVariables|GetActiveSegments)) 0.0 (Math|Conversions|ToFloat(Integer) (|(360-(360/NumSegments)) (Variables|Settings|GetSegments)))))
      (Spline|AddSplinePoint (Variables|Default|GetCircleSpline) (Math|Vector|MakeVector (* (Math|Trig|Sin(Degrees) (LocalVariables|GetSegmentOfCircumference)) (Variables|Settings|GetRadius)) (* (Math|Trig|Cos(Degrees) (LocalVariables|GetSegmentOfCircumference)) (Variables|Settings|GetRadius)) 0.0) "Local" false)))
  (Spline|UpdateSpline (Variables|Default|GetCircleSpline)))