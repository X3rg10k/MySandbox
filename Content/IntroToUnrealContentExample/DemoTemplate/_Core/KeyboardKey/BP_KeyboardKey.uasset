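; BP_KeyboardKey is a Blueprint that shows a keyboard key label through a widget component in the demo template.
; It casts the component's widget to UIE_KeyboardKey, passes in its Key value and sets the text to it.
; The same update runs in the Construction Script and again on BeginPlay, which also makes the widget visible.
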(event `self.ReceiveBeginPlay`
  (`SceneComponent.SetVisibility` (`self.Widget`) true false)
  (bind _asuie_keyboard_key (cast `/Game/IntroToUnrealContentExample/DemoTemplate/_Core/KeyboardKey/UIE_KeyboardKey` (`WidgetComponent.GetWidget` (`self.Widget`))))
  (bind _output_get (set `/Game/IntroToUnrealContentExample/DemoTemplate/_Core/KeyboardKey/UIE_KeyboardKey.Key` (`self.Key`) _asuie_keyboard_key))
  (`TextBlock.SetText` (`/Game/IntroToUnrealContentExample/DemoTemplate/_Core/KeyboardKey/UIE_KeyboardKey.Text` _asuie_keyboard_key) _output_get))

(fn `UserConstructionScript`
  (bind _asuie_keyboard_key (cast `/Game/IntroToUnrealContentExample/DemoTemplate/_Core/KeyboardKey/UIE_KeyboardKey` (`WidgetComponent.GetWidget` (`self.Widget`))))
  (bind _output_get (set `/Game/IntroToUnrealContentExample/DemoTemplate/_Core/KeyboardKey/UIE_KeyboardKey.Key` (`self.Key`) _asuie_keyboard_key))
  (`TextBlock.SetText` (`/Game/IntroToUnrealContentExample/DemoTemplate/_Core/KeyboardKey/UIE_KeyboardKey.Text` _asuie_keyboard_key) _output_get))